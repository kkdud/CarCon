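; Camera pawn with mouse look, wheel zoom and automatic depth-of-field focus.
; Axis inputs drive controller yaw and pitch, while the mouse wheel changes spring arm length within clamped limits.
; A looping timer runs a debug-drawn visibility trace and sets the camera's focal distance to the hit distance.
; The trace end is the scaled camera forward vector alone, not offset from the camera location.
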(event Custom|DoF
  (bind _camera (Variables|Default|GetCamera))
  (bind (_outhit _returnvalue) (Collision|LineTraceByChannel (Transformation|GetWorldLocation _camera) (* (Math|Vector|GetForwardVector _camera) 2e+03) "TraceTypeQuery1" false 0 "ForDuration" true "(R=1.000000,G=0.000000,B=0.000000,A=1.000000)" "(R=0.000000,G=1.000000,B=0.000000,A=1.000000)" 1.0))
  (if _returnvalue
    (Variables|Default|SetFocalLocation (Math|Vector|VectorLength (- (.Location (Collision|BreakHitResult _outhit)) (Transformation|GetWorldLocation (Variables|Default|GetCamera)))))
    (Variables|/Script/Engine.CameraComponent|SetPostProcessSettings (Variables|Default|GetCamera) (Utilities|Struct|MakePostProcessSettings 4.0 (Variables|Default|GetFocalLocation)))))

(event EventBeginPlay
  (Utilities|Time|SetTimerbyFunctionName 0 "DoF" 0.2 true))

(event Input|AxisEvents|InputAxisTurn
  (params (AxisValue :type Float%20%28single-precision%29))
  ;[1 1 1] Handle Input Event
  (Pawn|Input|AddControllerYawInput (* AxisValue 0.7)))

(event Input|AxisEvents|InputAxisLookUp
  (params (AxisValue :type Float%20%28single-precision%29))
  ;[1 1 1] Handle Input Event
  (Pawn|Input|AddControllerPitchInput (* AxisValue -0.7)))

(event Input|MouseEvents|MouseWheelUp
  (params (Key :type Key%20Structure :default "None"))
  ;[1 1 1] Handle Input Event
  (:Pressed
    (Variables|/Script/Engine.SpringArmComponent|SetTargetArmLength (Variables|Default|GetSpringArm) (Math|Float|Clamp(Float) (- (Variables|/Script/Engine.SpringArmComponent|GetTargetArmLength (Variables|Default|GetSpringArm)) 2e+01) 1e+02 5e+02))))

(event Input|MouseEvents|MouseWheelDown
  (params (Key :type Key%20Structure :default "None"))
  ;[1 1 1] Handle Input Event
  (:Pressed
    (Variables|/Script/Engine.SpringArmComponent|SetTargetArmLength (Variables|Default|GetSpringArm) (Math|Float|Clamp(Float) (+ (Variables|/Script/Engine.SpringArmComponent|GetTargetArmLength (Variables|Default|GetSpringArm)) 2e+01) 1e+02 5e+02))))

(fn ConstructionScript)