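; Car actor with a Control Rig body, convertible top and dashboard lights.
; Keys 1-3 switch red, blue or silver paint, with a timeline driving MPC_CarPaint's Time, then copying BaseColor_B into BaseColor_A.
; Helper functions snap rig bones to pivot components, set root and steering from a spline, and ease controls between poses.
; Others swap materials for warning lights and top parts hidden in the trunk, and toggle regular or cine top visibility.
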(event Input|KeyboardEvents|1
  (params (Key :type Key%20Structure :default "None"))
  (:Pressed
    (Utilities|MCRChangingPaint (Variables|Default|GetCarPaint_Red))
    (bind _newtrack_0 (Timeline|Timeline_0 PlayFromStart)
      (:Update
        (Rendering|Material|SetScalarParameterValue "/Game/Car/MPC_CarPaint.MPC_CarPaint" "Time" _newtrack_0 :!class /Script/Engine.KismetMaterialLibrary))
      (:Finished
        (bind _returnvalue (Rendering|Material|GetVectorParameterValue "/Game/Car/MPC_CarPaint.MPC_CarPaint" "BaseColor_B" :!class /Script/Engine.KismetMaterialLibrary))
        (Rendering|Material|SetVectorParameterValue "/Game/Car/MPC_CarPaint.MPC_CarPaint" "BaseColor_A" _returnvalue :!class /Script/Engine.KismetMaterialLibrary)))))

(event Input|KeyboardEvents|3
  (params (Key :type Key%20Structure :default "None"))
  (:Pressed
    (Utilities|MCRChangingPaint (Variables|Default|GetCarPaint_Silver))
    (bind _newtrack_0 (Timeline|Timeline_0 PlayFromStart)
      (:Update
        (Rendering|Material|SetScalarParameterValue "/Game/Car/MPC_CarPaint.MPC_CarPaint" "Time" _newtrack_0 :!class /Script/Engine.KismetMaterialLibrary))
      (:Finished
        (bind _returnvalue (Rendering|Material|GetVectorParameterValue "/Game/Car/MPC_CarPaint.MPC_CarPaint" "BaseColor_B" :!class /Script/Engine.KismetMaterialLibrary))
        (Rendering|Material|SetVectorParameterValue "/Game/Car/MPC_CarPaint.MPC_CarPaint" "BaseColor_A" _returnvalue :!class /Script/Engine.KismetMaterialLibrary)))))

(event Input|KeyboardEvents|2
  (params (Key :type Key%20Structure :default "None"))
  (:Pressed
    (Utilities|MCRChangingPaint (Variables|Default|GetCarPaint_Blue))
    (bind _newtrack_0 (Timeline|Timeline_0 PlayFromStart)
      (:Update
        (Rendering|Material|SetScalarParameterValue "/Game/Car/MPC_CarPaint.MPC_CarPaint" "Time" _newtrack_0 :!class /Script/Engine.KismetMaterialLibrary))
      (:Finished
        (bind _returnvalue (Rendering|Material|GetVectorParameterValue "/Game/Car/MPC_CarPaint.MPC_CarPaint" "BaseColor_B" :!class /Script/Engine.KismetMaterialLibrary))
        (Rendering|Material|SetVectorParameterValue "/Game/Car/MPC_CarPaint.MPC_CarPaint" "BaseColor_A" _returnvalue :!class /Script/Engine.KismetMaterialLibrary)))))

(fn ConstructionScript
  (Class|ControlRigComponent|AddMappedCompleteSkeletalMesh (Variables|Default|GetControlRig) (Variables|Default|GetSkeletalMesh)))

(fn RigSetup
  (bind _controlrig (Variables|Default|GetControlRig))
  ;[1 1 1] For each RigPrep object, find the corresponding ControlRig bone. Snap the bone to the RigPrep object location
  (for _array_element (Components|GetChildrenComponents (Variables|Default|Getpivots1) true)
    (Class|ControlRigComponent|SetInitialBoneTransform _controlrig (Utilities|String|StringToName (Utilities|String|LeftChop (Utilities|GetObjectName _array_element) 1)) (Transformation|GetWorldTransform _array_element) "WorldSpace" true)
    (Class|ControlRigComponent|SetBoneTransform _controlrig (Utilities|String|StringToName (Utilities|String|LeftChop (Utilities|GetObjectName _array_element) 1)) (Transformation|GetWorldTransform _array_element) "WorldSpace" 1.0 true)))

(fn SplineControl
  (bind _returnvalue (Actor|GetComponentbyClass "/Script/Engine.SplineComponent"))
  (bind _returnvalue_2 (Spline|GetTransformatDistanceAlongSpline _returnvalue 0.0 "World" false))
  (if (Utilities|IsValid 0)
    (Class|ControlRigComponent|SetControlTransform (Variables|Default|GetControlRig) "root_ctrl" (Math|Transform|ComposeTransforms (Math|Transform|MakeTransform (Math|Vector|MakeVector 0.0 0.0 0.0)) _returnvalue_2) "WorldSpace")
    (Class|ControlRigComponent|SetControlFloat (Variables|Default|GetControlRig) "Steering_CTRL" (* (.y (Math|Transform|InverseTransformLocation _returnvalue_2 (.location (Spline|GetTransformatDistanceAlongSpline _returnvalue (+ 0.0 1.0) "World" false)))) 1.0))))

(fn BlendControlRigInput
  (params (Control :type Name) (TargetRot :type Rotator) (IsOpen :type Boolean) (AnimationScale :type Float%20%28single-precision%29) (TargetPos :type Vector))
  (bind _returnvalue (Utilities|Time|GetWorldDeltaSeconds))
  (bind _returnvalue_2 (Utilities|Time|GetWorldDeltaSeconds))
  (bind _returnvalue_3 (* _returnvalue_2 AnimationScale))
  (bind _returnvalue_4 (* _returnvalue AnimationScale))
  (if IsOpen
    ;[1 1 1] Open Animation
    (Class|ControlRigComponent|SetControlTransform (Variables|Default|GetControlRig) Control (Math|Transform|MakeTransform (Math|Interpolation|Ease "EaseIn" _returnvalue_3 (Class|ControlRigComponent|GetControlPosition (Variables|Default|GetControlRig) Control "LocalSpace") TargetPos 1.0) (Math|Interpolation|Ease "EaseIn" _returnvalue_3 (Class|ControlRigComponent|GetControlRotator (Variables|Default|GetControlRig) Control "LocalSpace") TargetRot true 0.75) "1,1,1") "LocalSpace")
    (else
      ;[1 1 1] Close animation
      (Class|ControlRigComponent|SetControlTransform (Variables|Default|GetControlRig) Control (Math|Transform|MakeTransform (Math|Interpolation|Ease "ExpoOut" _returnvalue_4 (Class|ControlRigComponent|GetControlPosition (Variables|Default|GetControlRig) Control "LocalSpace") TargetPos) (Math|Interpolation|Ease "ExpoOut" _returnvalue_4 (Class|ControlRigComponent|GetControlRotator (Variables|Default|GetControlRig) Control "LocalSpace") TargetRot false) "1,1,1") "LocalSpace"))))

(fn IncreaseLEDs
  (params (DT :type Float%20%28single-precision%29))
  (Utilities|FlowControl|Sequence))

(fn DecreaseLEDs
  (params (DT :type Float%20%28single-precision%29))
  (Utilities|FlowControl|Sequence))

(fn AssignDynamicMaterials
  ;[1 1 1] Dashboard
  (Rendering|Material|SetMaterial (Variables|Default|GetSM_gaugeDisplay) 0 0)
  (Rendering|Material|SetMaterial (Variables|Default|GetSM_lightControls) 4 0)
  (Rendering|Material|SetMaterial (Variables|Default|GetSM_dialBack) 1 0)
  (Rendering|Material|SetMaterial (Variables|Default|GetSM_dialBack) 4 0)
  (Rendering|Material|SetMaterial (Variables|Default|GetSM_dialBack) 5 0)
  (Rendering|Material|SetMaterial (Variables|Default|GetSM_steeringwheel) 1 0)
  (Rendering|Material|SetMaterial (Variables|Default|GetSM_extraButtons) 3 0)
  ;[1 1 1] HMI
  (Rendering|Material|SetMaterial (Variables|Default|GetSM_HMI) 0 0)
  ;[1 1 1] Heating control
  (Rendering|Material|SetMaterial (Variables|Default|GetSM_heatingControl) 6 0)
  (Rendering|Material|SetMaterial (Variables|Default|GetSM_heatingControl) 8 0)
  (Rendering|Material|SetMaterial (Variables|Default|GetSM_heatingControl) 7 0)
  (Rendering|Material|SetMaterial (Variables|Default|GetSM_heatingControl) 3 0)
  (Rendering|Material|SetMaterial (Variables|Default|GetSM_heatingControl) 9 0)
  ;[1 1 1] Speed and tach
  (Rendering|Material|SetMaterial (Variables|Default|GetSM_tachNeedle) 1 0)
  (Rendering|Material|SetMaterial (Variables|Default|GetSM_speedNeedle) 3 0)
  ;[1 1 1] Center console
  (Rendering|Material|SetMaterial (Variables|Default|GetSM_centerconsoleControl) 5 0)
  (Rendering|Material|SetMaterial (Variables|Default|GetSM_centerconsoleControl) 8 0)
  (Rendering|Material|SetMaterial (Variables|Default|GetSM_centerconsoleControl) 12 0)
  ;[1 1 1] Front lights
  (Rendering|Material|SetMaterial (Variables|Default|GetSM_Iheadlightglass) 0 0)
  (Rendering|Material|SetMaterial (Variables|Default|GetSM_headlightBrowLight) 0 0)
  ;[1 1 1] taillights
  (Rendering|Material|SetMaterial (Variables|Default|GetSM_Brakeinnerglass) 0 0))

(fn UpdateAniminEditor
  (Components|SkeletalMesh|SetUpdateAnimationinEditor (Variables|Default|GetConvertibleTop) true))

(fn SwitchTopVisible
  (bind _convertibletopcine (Variables|Default|GetConvertibleTopCine))
  (bind _convertibletop (Variables|Default|GetConvertibleTop))
  (if true
    (Rendering|SetVisibility _convertibletop true true)
    (Rendering|SetVisibility _convertibletopcine false true)
    (else
      (Rendering|SetVisibility _convertibletopcine true true)
      (Rendering|SetVisibility _convertibletop false true))))

(fn HideinTrunk
  (if true
    (Rendering|Material|SetMaterial (Variables|Default|GetConvertibleTop) 15 "/Game/CarConfigurator/Car/ConvertibleTop/M_Hiding.M_Hiding")
    (Rendering|Material|SetMaterial (Variables|Default|GetConvertibleTop) 31 "/Game/CarConfigurator/Car/ConvertibleTop/M_Hiding.M_Hiding")
    (Rendering|Material|SetMaterial (Variables|Default|GetConvertibleTop) 7 "/Game/CarConfigurator/Car/ConvertibleTop/M_Hiding.M_Hiding")
    (Rendering|Material|SetMaterial (Variables|Default|GetConvertibleTop) 17 "/Game/CarConfigurator/Car/ConvertibleTop/M_Hiding.M_Hiding")
    (Rendering|Material|SetMaterial (Variables|Default|GetConvertibleTop) 27 "/Game/CarConfigurator/Car/ConvertibleTop/M_Hiding.M_Hiding")))

(fn ShowinTrunk
  (if true
    (Rendering|Material|SetMaterial (Variables|Default|GetConvertibleTop) 15 "/Game/CarConfigurator/Car/ConvertibleTop/MI_TextilePlain_Int.MI_TextilePlain_Int")
    (Rendering|Material|SetMaterial (Variables|Default|GetConvertibleTop) 31 "/Game/CarConfigurator/Car/ConvertibleTop/MI_Glass_Convertible.MI_Glass_Convertible")
    (Rendering|Material|SetMaterial (Variables|Default|GetConvertibleTop) 7 "/Game/CarConfigurator/Car/ConvertibleTop/MI_TextilePlain_Int.MI_TextilePlain_Int")
    (Rendering|Material|SetMaterial (Variables|Default|GetConvertibleTop) 17 "/Game/CarConfigurator/Car/ConvertibleTop/MI_Metal_Painted.MI_Metal_Painted")
    (Rendering|Material|SetMaterial (Variables|Default|GetConvertibleTop) 27 "/Game/CarConfigurator/Car/ConvertibleTop/MI_Metal_Painted.MI_Metal_Painted")))

(fn BlendControlRigInputDials
  (params (Control :type Name) (TargetRot :type Rotator) (IsOpen :type Boolean) (AnimationScale :type Float%20%28single-precision%29) (TargetPos :type Vector))
  ;[1 1 1] Open Animation
  (Class|ControlRigComponent|SetControlTransform (Variables|Default|GetControlRig) Control (Math|Transform|MakeTransform "0, 0, 0" (Math|Rotator|MakeRotator (Math|Float|Lerp (.roll (Class|ControlRigComponent|GetControlRotator (Variables|Default|GetControlRig) Control "LocalSpace")) (.roll TargetRot) (* (Utilities|Time|GetWorldDeltaSeconds) AnimationScale)) 0.0 0.0) "1,1,1") "LocalSpace"))

(fn SetWarningLights
  (params (InputVal :type Float%20%28single-precision%29))
  (bind _output_get (LocalVariables|SetInputValue InputVal))
  (if (Math|Boolean|ORBoolean (== _output_get 1.0) (== _output_get 4.0) (== _output_get 8.0))
    (LocalVariables|SetMaterialValue "/Game/CarConfigurator/Shared/Materials/MI_LED_YellowWarning.MI_LED_YellowWarning")
    (else
      (LocalVariables|SetMaterialValue "/Game/CarConfigurator/Shared/Materials/MI_LED_RedWarning.MI_LED_RedWarning")))
  (if (< (LocalVariables|GetInputValue) 0.0)
    (Rendering|Material|SetMaterial (Variables|Default|GetSM_WarningLights) (- (Math|Float|Truncate (* (LocalVariables|GetInputValue) -1.0)) 1) "/Game/References/AutomotiveMats/Materials/Interior/Plastic/MI_Plastic_Smooth_Grey.MI_Plastic_Smooth_Grey")
    (else
      (Rendering|Material|SetMaterial (Variables|Default|GetSM_WarningLights) (- (Math|Float|Truncate (LocalVariables|GetInputValue)) 1) (LocalVariables|GetMaterialValue)))))